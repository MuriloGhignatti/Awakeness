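; BP_PickupActor is a world pickup for an inventory item, configured by its ItemClass.
; The construction script reads that class's default ItemInfo to set the mesh, scale, position and pickup sphere radius, then enables physics on the mesh.
; Each tick the PickupArea sphere moves to the simulated mesh's location.
; Overlaps with actors tagged Player send messages adding or removing this pickup from that player's pickup list.
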(event `self.ReceiveTick`
  (params (DeltaSeconds :type "Float (single-precision)"))
  (`SceneComponent.K2_SetWorldLocation` (`self.PickupArea`) (`SceneComponent.K2_GetComponentLocation` (`self.ItemMesh`)) false false))

(event `self.PickupArea.OnComponentBeginOverlap`
  (params (OverlappedComponent :type "PrimitiveComponent Object Reference") (OtherActor :type "Actor Object Reference") (OtherComp :type "PrimitiveComponent Object Reference") (OtherBodyIndex :type Integer) (bFromSweep :type Boolean) (SweepResult :type "HitResult Structure (by ref)"))
  (if (`self.ActorHasTag` OtherActor "Player")
    (message `/Game/FirstPersonBP/Blueprints/INT_FirstPersonChar.Add to Pickup List` OtherActor self)))

(event `self.PickupArea.OnComponentEndOverlap`
  (params (OverlappedComponent :type "PrimitiveComponent Object Reference") (OtherActor :type "Actor Object Reference") (OtherComp :type "PrimitiveComponent Object Reference") (OtherBodyIndex :type Integer))
  (if (`self.ActorHasTag` OtherActor "Player")
    (message `/Game/FirstPersonBP/Blueprints/INT_FirstPersonChar.Remove From Pickup List` OtherActor self)))

(fn `UserConstructionScript`
  (bind (_id _iteminfo) (defaults `Object` (`self.ItemClass`)))
  (`StaticMeshComponent.SetStaticMesh` (`self.ItemMesh`) (`.PickupMesh` (break `ItemInfo` _iteminfo)))
  (`SceneComponent.SetRelativeScale3D` (`self.ItemMesh`) (`.MeshScale` (break `ItemInfo` _iteminfo)))
  (`SceneComponent.K2_SetRelativeLocation` (`self.ItemMesh`) (`.MeshPosition` (break `ItemInfo` _iteminfo)) false false)
  (`SphereComponent.SetSphereRadius` (`self.PickupArea`) (`.Radius` (break `ItemInfo` _iteminfo)) true)
  (`PrimitiveComponent.SetSimulatePhysics` (`self.ItemMesh`) true))